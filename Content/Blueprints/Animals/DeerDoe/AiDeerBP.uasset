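; AI doe deer that roams, grazes, rests and flees, and can be hunted and harvested for venison and hide.
; DecideNextAction picks behaviour from hunger, energy and flee flags, fed by self-calling delayed drain and regen events with randomized starting stats.
; Perceived stimuli or projectile hits trigger fleeing; body, vitals and heart hits add timer-driven bleedout, ending in ragdoll death.
; Grazing requires a downward trace finding a specific surface type.
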(event OnTargetPerceptionUpdated(AIPerception)
  (params (Actor :type Actor%20Object%20Reference) (Stimulus :type AI%20Stimulus%20Structure))
  ;[1 1 1] Detect Noise
  (if (not (Variables|Default|GetShouldRun?))
    (Variables|Default|SetShouldRun? (.bSuccessfullySensed (Utilities|Struct|BreakAIStimulus Stimulus)))
    (CallFunction|DecideNextAction true)))

(event OnComponentBeginOverlap(VitalsHB)
  (params (OverlappedComponent :type Primitive%20Component%20Object%20Reference) (OtherActor :type Actor%20Object%20Reference) (OtherComp :type Primitive%20Component%20Object%20Reference) (OtherBodyIndex :type Integer) (bFromSweep :type Boolean) (SweepResult :type Hit%20Result%20Structure%20%28by%20ref%29))
  ;[1 1 1] Damage/BleedOut
  (if (not (Variables|Damage|GetIsDead?))
    (Utilities|Casting|CastToFirstPersonProjectile OtherActor)
    (Variables|Damage|SetDamage 1.0)
    (CallFunction|DealDamage)
    (Variables|Damage|SetBleedoutTick 0.2)
    (Development|PrintString "Hit Vitals")
    (bind _returnvalue (Utilities|Time|SetTimerbyEvent (delegate Custom|Bleedout) 1.0 true))
    (if true
      (Utilities|Time|ClearandInvalidateTimerbyHandle (stale Collision|EventActorBeginOverlap _returnvalue)))
    (Development|PrintString (Utilities|String|ToString(Float) (Variables|Damage|GetHealth)))
    (if (Variables|Damage|GetIsDead?)
      (Utilities|Time|ClearandInvalidateTimerbyHandle (stale Collision|EventActorBeginOverlap _returnvalue))
      (Utilities|Time|ClearandInvalidateTimerbyHandle _returnvalue)
      (Utilities|Time|ClearandInvalidateTimerbyHandle (stale OnComponentBeginOverlap(HeartHB) _returnvalue))
      (CallFunction|Death)
      (Utilities|FlowControl|Delay (Math|Conversions|ToFloat(Integer) (Math|Random|RandomIntegerinRange 60 120)))
      (Actor|DestroyActor)
      (elif (Variables|Default|GetOutofCombat?)
        (Utilities|Time|ClearandInvalidateTimerbyHandle (stale Collision|EventActorBeginOverlap _returnvalue))
        (Utilities|Time|ClearandInvalidateTimerbyHandle _returnvalue)
        (Utilities|Time|ClearandInvalidateTimerbyHandle (stale OnComponentBeginOverlap(HeartHB) _returnvalue))))))

(event OnComponentBeginOverlap(HeartHB)
  (params (OverlappedComponent :type Primitive%20Component%20Object%20Reference) (OtherActor :type Actor%20Object%20Reference) (OtherComp :type Primitive%20Component%20Object%20Reference) (OtherBodyIndex :type Integer) (bFromSweep :type Boolean) (SweepResult :type Hit%20Result%20Structure%20%28by%20ref%29))
  ;[1 1 1] Damage/BleedOut
  (if (not (Variables|Damage|GetIsDead?))
    (Utilities|Casting|CastToFirstPersonProjectile OtherActor)
    (Variables|Damage|SetDamage 3.0)
    (CallFunction|DealDamage)
    (Variables|Damage|SetBleedoutTick 0.5)
    (Development|PrintString "Hit Heart")
    (bind _returnvalue (Utilities|Time|SetTimerbyEvent (delegate Custom|Bleedout) 1.0 true))
    (if true
      (Utilities|Time|ClearandInvalidateTimerbyHandle (stale OnComponentBeginOverlap(VitalsHB) _returnvalue)))
    (Development|PrintString (Utilities|String|ToString(Float) (Variables|Damage|GetHealth)))
    (if (Variables|Damage|GetIsDead?)
      (Utilities|Time|ClearandInvalidateTimerbyHandle (stale Collision|EventActorBeginOverlap _returnvalue))
      (Utilities|Time|ClearandInvalidateTimerbyHandle (stale OnComponentBeginOverlap(VitalsHB) _returnvalue))
      (Utilities|Time|ClearandInvalidateTimerbyHandle _returnvalue)
      (CallFunction|Death)
      (Utilities|FlowControl|Delay (Math|Conversions|ToFloat(Integer) (Math|Random|RandomIntegerinRange 60 120)))
      (Actor|DestroyActor)
      (elif (Variables|Default|GetOutofCombat?)
        (Utilities|Time|ClearandInvalidateTimerbyHandle (stale Collision|EventActorBeginOverlap _returnvalue))
        (Utilities|Time|ClearandInvalidateTimerbyHandle (stale OnComponentBeginOverlap(VitalsHB) _returnvalue))
        (Utilities|Time|ClearandInvalidateTimerbyHandle _returnvalue)))))

(event Custom|Decide%20Next%20Action
  (params (SkipDelay? :type Boolean))
  ;[1 1 1] Decide Next Action
  (if (not (Variables|Damage|GetIsDead?))
    (if SkipDelay?
      _
      (else
        (Utilities|FlowControl|Delay (Math|Conversions|ToFloat(Integer) (Math|Random|RandomIntegerinRange 1 5)))))
    (if (Variables|Default|GetShouldRun?)
      (CallFunction|RunAway)
      (elif (Variables|Hunger|GetIsHungry?)
        (CallFunction|Eat)
        (CallFunction|RegenHealth)
        (elif (Variables|Energy|GetIsTired?)
          (CallFunction|Rest)
          (CallFunction|RegainEnergy)
          (elif (not (Variables|Default|GetIsThirsty?))
            (CallFunction|RandomRoam)
            (CallFunction|OutOfCombat)))))))

(event Custom|Bleedout
  ;[1 1 1] Damage/BleedOut
  (CallFunction|BleedoutTick self)
  (Development|PrintString (Utilities|String|ToString(Float) (Variables|Damage|GetHealth)))
  (if (Variables|Damage|GetIsDead?)
    (Utilities|Time|ClearandInvalidateTimerbyHandle (stale Collision|EventActorBeginOverlap _returnvalue))
    (Utilities|Time|ClearandInvalidateTimerbyHandle (stale OnComponentBeginOverlap(VitalsHB) _returnvalue))
    (Utilities|Time|ClearandInvalidateTimerbyHandle (stale OnComponentBeginOverlap(HeartHB) _returnvalue))
    (CallFunction|Death)
    (Utilities|FlowControl|Delay (Math|Conversions|ToFloat(Integer) (Math|Random|RandomIntegerinRange 60 120)))
    (Actor|DestroyActor)
    (elif (Variables|Default|GetOutofCombat?)
      (Utilities|Time|ClearandInvalidateTimerbyHandle (stale Collision|EventActorBeginOverlap _returnvalue))
      (Utilities|Time|ClearandInvalidateTimerbyHandle (stale OnComponentBeginOverlap(VitalsHB) _returnvalue))
      (Utilities|Time|ClearandInvalidateTimerbyHandle (stale OnComponentBeginOverlap(HeartHB) _returnvalue)))))

(event Custom|Add%20Hunger
  ;[1 1 1] HungerGain
  (if (Variables|Hunger|GetIsHungry?)
    (bind _output_get (Variables|Hunger|SetHunger (Math|Integer|Clamp(Integer) (+ (Variables|Hunger|GetHunger) (Variables|Hunger|GetHungerGain)) 0 (Variables|Hunger|GetMaxHunger))))
    (if (not (== _output_get (Variables|Hunger|GetMaxHunger)))
      (Utilities|FlowControl|Delay 1.0)
      (CallFunction|AddHunger))))

(event Custom|Regen%20Health
  ;[1 1 1] Regain Health
  (if (and (< (Variables|Damage|GetHealth) (Variables|Damage|GetMax%20Health)) (not (Variables|Default|GetShouldRun?)))
    (bind _output_get (Variables|Damage|SetHealth (Math|Float|Clamp(Float) (+ (Variables|Damage|GetHealth) (Variables|Damage|GetHealthGain)) 0.0 (Variables|Damage|GetMax%20Health))))
    (if (not (== _output_get (Variables|Damage|GetMax%20Health)))
      (Utilities|FlowControl|Delay 1.0)
      (CallFunction|RegenHealth))))

(event Custom|Out%20of%20Combat
  ;[1 1 1] Regain Health
  (if (and (< (Variables|Damage|GetHealth) (Variables|Damage|GetMax%20Health)) (not (Variables|Default|GetShouldRun?)))
    (Utilities|FlowControl|Delay 5.0)
    (Variables|Default|SetOutofCombat? true)
    (CallFunction|RegenHealth)))

(event Custom|GoHome
  ;[1 1 1] Go Home & Sleep
  (AI|AIMoveTo self (Variables|Default|GetHome%20Location) 0 5.0 false
    (:OnSuccess
      (if (Variables|Energy|GetIsTired?)
        (CallFunction|Rest)
        (CallFunction|RegainEnergy)
        (else
          (CallFunction|DecideNextAction false))))))

(event Custom|Check%20If%20Dead
  (if (Variables|Damage|GetIsDead?)
    (CallFunction|Death)
    (Utilities|Time|ClearandInvalidateTimerbyHandle (stale EventBeginPlay _returnvalue))))

(event Custom|Random%20Roam
  ;[1 1 1] Random Roam
  (Variables|/Script/Engine.CharacterMovementComponent|SetMaxWalkSpeed (Variables|Character|GetCharacterMovement) 1e+02)
  (AI|AIMoveTo self (.RandomLocation (AI|Navigation|GetRandomReachablePointinRadius (Transformation|GetActorLocation) 1.5e+03 0 0)) 0 5.0 false
    (:OnSuccess
      (CallFunction|DecideNextAction false))))

(event Custom|Run%20Away
  ;[1 1 1] Run Away
  (CallFunction|StopAnimation)
  (Variables|/Script/Engine.CharacterMovementComponent|SetMaxWalkSpeed (Variables|Character|GetCharacterMovement) 6e+02)
  (AI|AIMoveTo self (.RandomLocation (AI|Navigation|GetRandomReachablePointinRadius (Transformation|GetActorLocation) (Math|Random|RandomFloatinRange 5e+04 1e+05) 0 0)) 0 5.0 false
    (:OnSuccess
      (Variables|Default|SetShouldRun? false)
      (CallFunction|DecideNextAction true))))

(event Custom|Rest
  ;[1 1 1] Sleeping Anim
  (Components|Movement|StopMovementImmediately (Variables|Character|GetCharacterMovement))
  (CallFunction|PlayAnimation "/Game/AnimalVarietyPack/DeerStagAndDoe/Animations/ANIM_DeerDoe_GoToRest.ANIM_DeerDoe_GoToRest" false)
  (Utilities|FlowControl|Delay 1.4)
  (CallFunction|PlayAnimation "/Game/AnimalVarietyPack/DeerStagAndDoe/Animations/ANIM_DeerDoe_IdleRest.ANIM_DeerDoe_IdleRest" true)
  (Utilities|FlowControl|Delay (Math|Conversions|ToFloat(Integer) (Math|Random|RandomIntegerinRange 50 120)))
  (CallFunction|PlayAnimation "/Game/AnimalVarietyPack/DeerStagAndDoe/Animations/ANIM_DeerDoe_RestToGoBackUp.ANIM_DeerDoe_RestToGoBackUp" false)
  (Utilities|FlowControl|Delay 1.4)
  (CallFunction|StopAnimation)
  (Variables|Energy|SetIsTired? false)
  (CallFunction|DecideNextAction false)
  (CallFunction|DrainEnergy))

(event Custom|DrainEnergy
  ;[1 1 1] Drain Energy - Normal = 125 sec
  (if (not (Variables|Energy|GetIsTired?))
    (bind _output_get (Variables|Energy|SetEnergy (Math|Integer|Clamp(Integer) (- (Variables|Energy|GetEnergy) (Variables|Energy|GetEnergyDrain)) 0 (Variables|Energy|GetMaxEnergy))))
    (if (== _output_get 0)
      (Variables|Energy|SetIsTired? true)
      (CallFunction|DecideNextAction false)
      (else
        (Utilities|FlowControl|Delay 1.0)
        (CallFunction|DrainEnergy)))))

(event Custom|Regain%20Energy
  ;[1 1 1] Regain Energy - Normal = 50 sec
  (if (Variables|Energy|GetIsTired?)
    (bind _output_get (Variables|Energy|SetEnergy (Math|Integer|Clamp(Integer) (+ (Variables|Energy|GetEnergy) (Variables|Energy|GetEnergy%20Gain)) 0 (Variables|Energy|GetMaxEnergy))))
    (if (not (== _output_get (Variables|Energy|GetMaxEnergy)))
      (Utilities|FlowControl|Delay 1.0)
      (CallFunction|RegainEnergy))))

(event Custom|Drain%20Hunger
  ;[1 1 1] Drain Hunger
  (if (not (Variables|Hunger|GetIsHungry?))
    (bind _output_get (Variables|Hunger|SetHunger (Math|Integer|Clamp(Integer) (- (Variables|Hunger|GetHunger) (Variables|Hunger|GetHungerDrain)) 0 (Variables|Hunger|GetMaxHunger))))
    (if (== _output_get 0)
      (Variables|Hunger|SetIsHungry? true)
      (CallFunction|DecideNextAction false)
      (else
        (Utilities|FlowControl|Delay 1.0)
        (CallFunction|DrainHunger)))))

(event Custom|Eat
  ;[1 1 1] Eat Animation
  (bind _caneat_ (Utilities|CanEat)
    (:Out
      (if _caneat_
        (Components|Movement|StopMovementImmediately (Variables|Character|GetCharacterMovement))
        (CallFunction|AddHunger)
        (CallFunction|PlayAnimation "/Game/AnimalVarietyPack/DeerStagAndDoe/Animations/ANIM_DeerDoe_GrazeOnce.ANIM_DeerDoe_GrazeOnce" false)
        (Utilities|FlowControl|Delay 1.0)
        (CallFunction|PlayAnimation "/Game/AnimalVarietyPack/DeerStagAndDoe/Animations/ANIM_DeerDoe_IdleGraze.ANIM_DeerDoe_IdleGraze" true)
        (Utilities|FlowControl|Delay (Math|Conversions|ToFloat(Integer) (Math|Random|RandomIntegerinRange 3 10)))
        (CallFunction|PlayAnimation "/Game/AnimalVarietyPack/DeerStagAndDoe/Animations/ANIM_DeerDoe_Graze_End.ANIM_DeerDoe_Graze_End" false)
        (Utilities|FlowControl|Delay 1.0)
        (CallFunction|StopAnimation)
        (Variables|Hunger|SetIsHungry? false)
        (CallFunction|DrainHunger)
        (CallFunction|DecideNextAction false)
        (else
          (CallFunction|DecideNextAction false)
          (Variables|Hunger|SetIsHungry? false)
          (Utilities|FlowControl|Delay 5.0)
          (Variables|Hunger|SetIsHungry? true))))))

(event Custom|Deal%20Damage
  ;[1 1 1] Take Damage
  (if (not (Variables|Damage|GetIsDead?))
    (bind _output_get (Variables|Damage|SetHealth (Math|Float|Clamp(Float) (- (Variables|Damage|GetHealth) (Variables|Damage|GetDamage)) 0.0 (Variables|Damage|GetMax%20Health))))
    (Audio|PlaySoundatLocation "/Game/Blueprints/Sounds/Animal/Deer/DeerMewCue.DeerMewCue" (Transformation|GetActorLocation) "0, 0, 0" 1.0 1.0 0.0 0 0 0)
    (if (== _output_get 0.0)
      (CallFunction|Death)
      (Utilities|FlowControl|Delay (Math|Conversions|ToFloat(Integer) (Math|Random|RandomIntegerinRange 60 120)))
      (Actor|DestroyActor)
      (else
        (Components|Movement|StopMovementImmediately (Variables|Character|GetCharacterMovement))
        (CallFunction|PlayAnimation "/Game/AnimalVarietyPack/DeerStagAndDoe/Animations/ANIM_DeerDoe_GetHit.ANIM_DeerDoe_GetHit" false)
        (Variables|Default|SetShouldRun? true)
        (Variables|Default|SetOutofCombat? false)
        (Utilities|FlowControl|Delay 0.7)
        (CallFunction|StopAnimation)
        (if (not (Variables|Damage|GetIsDead?))
          (CallFunction|DecideNextAction true))))))

(event EventBeginPlay
  (bind _returnvalue (Utilities|Time|SetTimerbyEvent (delegate Custom|Check%20If%20Dead) 0.05 true))
  (CallFunction|DecideNextAction false)
  (CallFunction|DrainEnergy)
  (CallFunction|DrainHunger))

(event Collision|EventActorBeginOverlap
  (params (OtherActor :type Actor%20Object%20Reference))
  ;[1 1 1] Damage/BleedOut
  (if (not (Variables|Damage|GetIsDead?))
    (Utilities|Casting|CastToFirstPersonProjectile OtherActor)
    (Variables|Damage|SetDamage 0.5)
    (CallFunction|DealDamage)
    (Variables|Damage|SetBleedoutTick 0.1)
    (Development|PrintString "Hit")
    (bind _returnvalue (Utilities|Time|SetTimerbyEvent (delegate Custom|Bleedout) 0.5 true))
    (if true
      (Development|PrintString (Utilities|String|ToString(Float) (Variables|Damage|GetHealth)))
      (if (Variables|Damage|GetIsDead?)
        (Utilities|Time|ClearandInvalidateTimerbyHandle _returnvalue)
        (Utilities|Time|ClearandInvalidateTimerbyHandle (stale OnComponentBeginOverlap(VitalsHB) _returnvalue))
        (Utilities|Time|ClearandInvalidateTimerbyHandle (stale OnComponentBeginOverlap(HeartHB) _returnvalue))
        (CallFunction|Death)
        (Utilities|FlowControl|Delay (Math|Conversions|ToFloat(Integer) (Math|Random|RandomIntegerinRange 60 120)))
        (Actor|DestroyActor)
        (elif (Variables|Default|GetOutofCombat?)
          (Utilities|Time|ClearandInvalidateTimerbyHandle _returnvalue)
          (Utilities|Time|ClearandInvalidateTimerbyHandle (stale OnComponentBeginOverlap(VitalsHB) _returnvalue))
          (Utilities|Time|ClearandInvalidateTimerbyHandle (stale OnComponentBeginOverlap(HeartHB) _returnvalue)))))))

(event EventInteract
  (params (Interacter :type First%20Person%20Character%20Object%20Reference))
  (bind _inventorycomponent (Variables|/Game/Blueprints/FirstPersonBP/Blueprints/FirstPersonCharacter.FirstPersonCharacter_C|GetInventoryComponent Interacter))
  ;[1 1 1] Gather Meat
  (if (not (Variables|Default|GetConsumed))
    (if (Variables|Damage|GetIsDead?)
      (bind _success (Default|AddtoInventory _inventorycomponent "/Game/Blueprints/Item/Item_Venison.Item_Venison_C" 3))
      (bind _success_2 (Default|AddtoInventory _inventorycomponent "/Game/Blueprints/Item/Item_DeerSkin.Item_DeerSkin_C" 2))
      (if (and _success_2 _success)
        (bind _asmy_player_controller (Utilities|Casting|CastToMyPlayerController (Game|GetPlayerController 0)))
        (Default|RefreshInventory (Variables|/Game/Blueprints/UI/HUD.HUD_C|GetInventoryWindow (Variables|/Game/Blueprints/UI/MyPlayerController.MyPlayerController_C|GetHUD%20Widget _asmy_player_controller)))
        (Default|RefreshInventory (Variables|/Game/Blueprints/UI/HUD.HUD_C|GetCraftingMenu (Variables|/Game/Blueprints/UI/MyPlayerController.MyPlayerController_C|GetHUD%20Widget _asmy_player_controller)))
        (Variables|Default|SetConsumed true)))))

(event EventDestroyed
  (Utilities|Array|RemoveItem (Variables|/Game/Blueprints/Animals/BP_SpawnPoint.BP_SpawnPoint_C|GetActivePawns (Variables|Default|GetSpawnPoint)) self))

(fn ConstructionScript
  (Variables|Energy|SetMaxEnergy (Math|Integer|Clamp(Integer) (Math|Random|RandomIntegerinRange 250 350) 250 350))
  (Variables|Energy|SetEnergy (Math|Integer|Clamp(Integer) (Math|Random|RandomIntegerinRange 0 (Variables|Energy|GetMaxEnergy)) 0 (Variables|Energy|GetMaxEnergy)))
  (Variables|Hunger|SetMaxHunger (Math|Integer|Clamp(Integer) (Math|Random|RandomIntegerinRange 225 350) 225 350))
  (Variables|Hunger|SetHunger (Math|Integer|Clamp(Integer) (Math|Random|RandomIntegerinRange 0 (Variables|Hunger|GetMaxHunger)) 0 (Variables|Hunger|GetMaxHunger)))
  (Variables|Damage|SetMax%20Health (Math|Float|Clamp(Float) (Math|Random|RandomFloatinRange 1e+01 1e+01) 1e+01 1e+01))
  (Variables|Damage|SetHealth (Math|Float|Clamp(Float) (Math|Random|RandomFloatinRange (/ (Variables|Damage|GetMax%20Health) 0.5) (Variables|Damage|GetMax%20Health)) 1.0 (Variables|Damage|GetMax%20Health))))

(fn Death
  (bind _charactermovement (Variables|Character|GetCharacterMovement))
  (Components|Movement|StopMovementImmediately _charactermovement)
  (Pawn|Components|CharacterMovement|DisableMovement _charactermovement)
  (Variables|Damage|SetHealth 0.0)
  (Variables|Damage|SetIsDead? true)
  (Components|Animation|PlayAnimation (Variables|Character|GetMesh) "/Game/AnimalVarietyPack/DeerStagAndDoe/Animations/ANIM_DeerDoe_Death.ANIM_DeerDoe_Death" false)
  (CallFunction|Ragdoll))

(fn BleedoutTick
  (Variables|Damage|SetHealth (Math|Float|Clamp(Float) (- (Variables|Damage|GetHealth) (Variables|Damage|GetBleedoutTick)) 0.0 (Variables|Damage|GetMax%20Health)))
  (if (<= (Variables|Damage|GetHealth) 0.0)
    (Variables|Damage|SetIsDead? true))
  (return))

(fn PlayAnimation
  (params (Animation :type Animation%20Asset%20Object%20Reference) (ShouldLoop? :type Boolean))
  (Components|Animation|PlayAnimation (Variables|Character|GetMesh) Animation ShouldLoop?))

(fn StopAnimation
  (bind _mesh (Variables|Character|GetMesh))
  (Components|Animation|SetAnimationMode _mesh "AnimationBlueprint")
  (Class|SkeletalMeshComponent|SetAnimClass _mesh "/Game/Blueprints/Animals/DeerDoe/AiDeerDoeAnimBP.AiDeerDoeAnimBP_C"))

(fn Ragdoll
  (Physics|SetSimulatePhysics (Variables|Character|GetMesh) true)
  (Pawn|Components|CharacterMovement|DisableMovement (Variables|Character|GetCharacterMovement)))