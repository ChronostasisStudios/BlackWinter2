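; Weather manager that runs the day/night cycle and world temperature, with days shortening and cooling as they pass.
; Tick advances elapsed time, rotates the sun, updates the sky sphere and HUD clock, and fades sun and skylight by night state, polled in a delay loop.
; Looping timers compute temperature from a daily curve plus random variation and apply daily seasonal drift.
; Start day offsets initial daylight hours and base temperature.
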(event EventBeginPlay
  (Utilities|FlowControl|Sequence
    (:then_0
      (DayNightCycle|GetSunandSky))
    (:then_1
      (DayNightCycle|SetSunIntensity))
    (:then_2
      (Time|SetElapsedTimeBasedonStartTime))
    (:then_3
      (Temperature|StartUpdatingTemperature))
    (:then_4
      (Time|SetTimeOfYear))
    (:then_5
      (DayNightCycle|DetermineifNight :!label _label)
      (Utilities|FlowControl|Delay 0.05)
      (goto _label))))

(event EventTick
  (params (DeltaSeconds :type Float%20%28single-precision%29))
  (Utilities|FlowControl|Sequence
    (:then_0
      (Time|UpdateElapsedTime))
    (:then_1
      (DayNightCycle|UpdateSunPosition))
    (:then_2
      (Time|UpdateCurrentTime))
    (:then_3
      (DayNightCycle|FadeSun))))

(fn ConstructionScript
  (Variables|Time|SetSecondsPerDay (* (Variables|Time|GetMinutesPerDay) 6e+01)))

(fn GetSunandSky
  (Utilities|IsValid (Variables|DayNightCycle|GetSun)
    (:Is%20Valid
      _)
    (:Is%20Not%20Valid
      (bind _outactors (Actor|GetAllActorsOfClass "/Script/Engine.DirectionalLight"))
      (Variables|DayNightCycle|SetSun (Utilities|Array|Get(acopy) _outactors))))
  (Utilities|IsValid (Variables|DayNightCycle|GetSky)
    (:Is%20Valid
      _)
    (:Is%20Not%20Valid
      (bind _outactors_2 (Actor|GetAllActorsOfClass "/Engine/EngineSky/BP_Sky_Sphere.BP_Sky_Sphere_C"))
      (Variables|DayNightCycle|SetSky (Utilities|Array|Get(acopy) _outactors_2))))
  (Utilities|IsValid (Variables|DayNightCycle|GetSkyLight)
    (:Is%20Not%20Valid
      (bind _outactors_3 (Actor|GetAllActorsOfClass "/Script/Engine.SkyLight"))
      (Variables|DayNightCycle|SetSkyLight (Utilities|Array|Get(acopy) _outactors_3)))))

(fn SetSunIntensity
  (Variables|DayNightCycle|SetSunIntensity (Variables|/Script/Engine.LightComponentBase|GetIntensity (Variables|/Script/Engine.Light|GetLightComponent (Variables|DayNightCycle|GetSun))))
  (Variables|DayNightCycle|SetLightIntensity (Variables|/Script/Engine.LightComponentBase|GetIntensity (Variables|/Script/Engine.SkyLight|GetLightComponent (Variables|DayNightCycle|GetSkyLight)))))

(fn SetElapsedTimeBasedonStartTime
  (Variables|Time|SetElapsedTime (* (Time|GetTimeasSeconds (Variables|Time|GetStartTime)) (/ (Variables|Time|GetSecondsPerDay) 8.64e+04))))

(fn GetTimeasSeconds
  (params (Time :type F%20Time%20Structure%20%28by%20ref%29))
  (bind (_days _hours _minutes) (Utilities|Struct|BreakFTime Time))
  (return (+ (* _days 86400) (* _hours 3600) (* _minutes 60))))

(fn UpdateSunPosition
  (Transformation|SetRelativeRotation (Variables|/Script/Engine.Light|GetLightComponent (Variables|DayNightCycle|GetSun)) (Math|Rotator|MakeRotator 0.0 (+ (* (Time|GetFractionOfDay) -3.6e+02) 9e+01) 1.6e+02) false false)
  (Default|UpdateSunDirection (Variables|DayNightCycle|GetSky)))

(fn GetFractionOfDay
  (return (/ (Variables|Time|GetElapsedTime) (Variables|Time|GetSecondsPerDay))))

(fn UpdateElapsedTime
  (Variables|Time|SetElapsedTime (+ (Variables|Time|GetElapsedTime) (Utilities|Time|GetWorldDeltaSeconds))))

(fn UpdateCurrentTime
  (bind _output_get (Variables|Time|SetCurrentTime (Time|DetermineCurrentTime)))
  (bind _asfirst_person_character (Utilities|Casting|CastToFirstPersonCharacter (Game|GetPlayerCharacter 0)))
  (Default|SetTime (Variables|/Game/Blueprints/FirstPersonBP/Blueprints/FirstPersonCharacter.FirstPersonCharacter_C|GetPlayerUIHUD _asfirst_person_character) _output_get (Variables|Time|GetClockType)))

(fn DetermineCurrentTime
  (bind _return_value (Time|GetFractionOfDay))
  (return (Utilities|Struct|MakeFTime (Math|Float|Truncate _return_value) (Math|Float|Truncate (* (Math|Float|%(Float) _return_value 1.0) 24.0)) (Math|Float|Truncate (Math|Float|%(Float) (* _return_value 1.44e+03) 6e+01)))))

(fn DetermineifNight
  (bind _currenttime (Variables|Time|GetCurrentTime))
  (if (or (< (.hours _currenttime) (Math|Float|Truncate (Variables|Time|GetSunUpTime))) (>= (.hours _currenttime) (Math|Float|Truncate (Variables|Time|GetSunDownTime))))
    (Variables|DayNightCycle|SetIsNight? true)
    (else
      (Variables|DayNightCycle|SetIsNight? false)))
  (return false))

(fn FadeSun
  (bind _sun (Variables|DayNightCycle|GetSun))
  (bind _skylight (Variables|DayNightCycle|GetSkyLight))
  (bind _lightcomponent (Variables|/Script/Engine.Light|GetLightComponent _sun))
  (bind _lightcomponent_2 (Variables|/Script/Engine.SkyLight|GetLightComponent _skylight))
  (Rendering|Components|Light|SetIntensity _lightcomponent (Math|Float|Clamp(Float) (+ (Variables|/Script/Engine.LightComponentBase|GetIntensity _lightcomponent) (* (Utilities|Time|GetWorldDeltaSeconds) (/ 24.0 (Variables|Time|GetSecondsPerDay)) (Variables|DayNightCycle|GetSunIntensity) (select (Variables|DayNightCycle|GetIsNight?) -1.0 1.0))) 0.0 (Variables|DayNightCycle|GetSunIntensity)))
  (Rendering|Components|Light|SetIntensity _lightcomponent_2 (Math|Float|Clamp(Float) (+ (* (Utilities|Time|GetWorldDeltaSeconds) (/ 24.0 (Variables|Time|GetSecondsPerDay)) (Variables|DayNightCycle|GetLightIntensity) (select (Variables|DayNightCycle|GetIsNight?) -1.0 1.0)) (Variables|/Script/Engine.LightComponentBase|GetIntensity _lightcomponent_2)) 0.0 (Variables|DayNightCycle|GetLightIntensity))))

(fn StartUpdatingTemperature
  (Utilities|Time|SetTimerbyFunctionName self "UpdateWorldTemperature" (/ 1.0 (Variables|Temperature|GetTemperatureUpdateRate)) true)
  (Utilities|Time|SetTimerbyFunctionName self "TemperatureOverDays" (* (Variables|Time|GetMinutesPerDay) 6e+01) true)
  (Utilities|Time|SetTimerbyFunctionName self "ChangeLengthofDay" (* (Variables|Time|GetMinutesPerDay) 6e+01) true)
  (Utilities|Time|SetTimerbyFunctionName self "SetRandVariation" (* (Variables|Time|GetMinutesPerDay) 6e+01) true))

(fn UpdateWorldTemperature
  (bind _output_get (CallFunction|StoreWorldTemp))
  (Variables|Temperature|SetFinalWorldTemperature _output_get))

(fn SetHUDReference
  (bind _asfirst_person_character (Utilities|Casting|CastToFirstPersonCharacter (Game|GetPlayerCharacter 0)))
  (Variables|Default|SetCharacterHUDRef (Variables|/Game/Blueprints/FirstPersonBP/Blueprints/FirstPersonCharacter.FirstPersonCharacter_C|GetPlayerUIHUD _asfirst_person_character)))

(fn TemperatureOverDays
  (bind _currenttime (Variables|Time|GetCurrentTime))
  (if (> (.days _currenttime) 0)
    (if (> (.days _currenttime) 30)
      (Variables|Temperature|SetBaseWorldTemperature (- (Variables|Temperature|GetBaseWorldTemperature) 0.3))
      (else
        (Variables|Temperature|SetBaseWorldTemperature (- (Variables|Temperature|GetBaseWorldTemperature) 0.15))))
    (else
      (Variables|Temperature|SetBaseWorldTemperature (Variables|Temperature|GetBaseWorldTemperature))))
  (return))

(fn ChangeLengthofDay
  (if (> (.days (Variables|Time|GetCurrentTime)) 0)
    (bind _output_get (Variables|Time|SetSunUpTime (+ (Variables|Time|GetSunUpTime) 0.017)))
    (bind _output_get_2 (Variables|Time|SetSunDownTime (- (Variables|Time|GetSunDownTime) 0.017)))
    (Development|PrintString (Utilities|String|ToString(Float) _output_get))
    (Development|PrintString (Utilities|String|ToString(Float) _output_get_2))
    (else
      (Variables|Time|SetSunUpTime (Variables|Time|GetSunUpTime))
      (Variables|Time|SetSunDownTime (Variables|Time|GetSunDownTime)))))

(fn SetTimeOfYear
  (bind _starttime (Variables|Time|GetStartTime))
  (bind _returnvalue (* (.days _starttime) 0.017))
  (if (> (.days _starttime) 0)
    (Variables|Time|SetSunUpTime (+ (Variables|Time|GetSunUpTime) _returnvalue))
    (Variables|Time|SetSunDownTime (- (Variables|Time|GetSunDownTime) _returnvalue))
    (if (> (.days _starttime) 30)
      (if (> (.days _starttime) 55)
        (Variables|Temperature|SetBaseWorldTemperature 8.0)
        (else
          (Variables|Temperature|SetBaseWorldTemperature (- (Variables|Temperature|GetBaseWorldTemperature) (* (.days _starttime) 0.3)))))
      (else
        (Variables|Temperature|SetBaseWorldTemperature (- (Variables|Temperature|GetBaseWorldTemperature) (* (.days _starttime) 0.15)))))
    (else
      (Variables|Time|SetSunUpTime (Variables|Time|GetSunUpTime))
      (Variables|Time|SetSunDownTime (Variables|Time|GetSunDownTime))
      (Variables|Temperature|SetBaseWorldTemperature (Variables|Temperature|GetBaseWorldTemperature)))))

(fn SetRandVariation
  (bind _output_get (Variables|Temperature|SetRandVariation (Math|Random|RandomFloatinRange -2.0 2.0)))
  (return _output_get))

(fn StoreWorldTemp
  (bind _output_get (Variables|Temperature|SetStoredWorldTemp (+ (* (Math|Curves|GetFloatValue (Variables|Temperature|GetTempFluctuationCurve) (Math|Float|%(Float) (Time|GetFractionOfDay) 1.0)) (+ (Variables|Temperature|GetWorldTemperatureVariation) (Variables|Temperature|GetRandVariation))) (Variables|Temperature|GetBaseWorldTemperature))))
  (return _output_get))