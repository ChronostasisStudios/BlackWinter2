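; DynamicWeather_BP is a weather actor containing an unfinished transition from clear blue sky to dark overcast.
; A timeline drives lerps of the sky material's zenith, horizon and cloud colors, raises cloud opacity, and fades the referenced light from white to black.
; That chain is disconnected and never runs.
; BeginPlay only makes a non-looping, zero-time timer call bound to an empty custom event, so the weather never changes.
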(event Custom|CustomEvent_0)

(event EventBeginPlay
  (Utilities|Time|SetTimerbyEvent (delegate Custom|CustomEvent_0) 0.0))

(event Collision|EventActorBeginOverlap
  (params (OtherActor :type Actor%20Object%20Reference)))

(event EventTick
  (params (DeltaSeconds :type Float%20%28single-precision%29)))

(event Input|MouseEvents|LeftMouseButton
  (params (Key :type Key%20Structure :default "None")))

(fn ConstructionScript)