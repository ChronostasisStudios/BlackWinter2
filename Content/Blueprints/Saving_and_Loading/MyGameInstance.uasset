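; Game instance that manages save slots for the player's location, camera rotation, health, protein and water.
; LoadGame loads the named slot and starts a looping AutoSave timer, or creates a fresh save object without starting the timer if none exists.
; Save and load functions copy data between the first-person character and the cached save object.
; Other functions delete the current slot or read any slot's player data without replacing the cache.
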(event Custom|LoadGame
  (params (SaveSlotName :type String))
  (bind _output_get (Variables|Default|SetSaveSlotName SaveSlotName))
  (bind _returnvalue (SaveGame|DoesSaveGameExist _output_get))
  (if _returnvalue
    (bind _returnvalue_2 (SaveGame|LoadGamefromSlot (Variables|Default|GetSaveSlotName)))
    (bind _assave_game_object (Utilities|Casting|CastToSaveGameObject _returnvalue_2))
    (Variables|Default|SetSaveGameData _assave_game_object)
    (Utilities|Time|SetTimerbyFunctionName self "AutoSave" 5.0 true)
    (else
      (bind _returnvalue_3 (SaveGame|CreateSaveGameObject "/Game/Blueprints/Saving_and_Loading/SaveGameObject.SaveGameObject_C"))
      (Variables|Default|SetSaveGameData _returnvalue_3))))

(event EventInit)

(fn SavePlayerData
  (bind _asfirst_person_character (Utilities|Casting|CastToFirstPersonCharacter (Game|GetPlayerCharacter 0)))
  (bind _output_get (Variables|Default|SetPlayer%20Ref _asfirst_person_character))
  (Variables|/Game/Blueprints/Saving_and_Loading/SaveGameObject.SaveGameObject_C|SetPlayerData (Variables|Default|GetSaveGameData) (Utilities|Struct|MakePlayerSaveData (Transformation|GetActorLocation _output_get) (Variables|/Game/Blueprints/FirstPersonBP/Blueprints/FirstPersonCharacter.FirstPersonCharacter_C|GetHealth _output_get) (Variables|/Game/Blueprints/FirstPersonBP/Blueprints/FirstPersonCharacter.FirstPersonCharacter_C|GetProtein _output_get) (Variables|/Game/Blueprints/FirstPersonBP/Blueprints/FirstPersonCharacter.FirstPersonCharacter_C|GetWater _output_get) (Transformation|GetWorldRotation (Variables|/Game/Blueprints/FirstPersonBP/Blueprints/FirstPersonCharacter.FirstPersonCharacter_C|GetFirstPersonCamera _output_get))))
  (SaveGame|SaveGametoSlot (Variables|Default|GetSaveGameData) (Variables|Default|GetSaveSlotName)))

(fn LoadPlayerData
  (bind _asfirst_person_character (Utilities|Casting|CastToFirstPersonCharacter (Game|GetPlayerCharacter 0)))
  (bind _output_get (Variables|Default|SetPlayerRef _asfirst_person_character))
  (bind _savegamedata (Variables|Default|GetSaveGameData)
    (:then
      (Transformation|SetWorldRotation (Variables|/Game/Blueprints/FirstPersonBP/Blueprints/FirstPersonCharacter.FirstPersonCharacter_C|GetFirstPersonCamera _output_get) (.rotation (Variables|/Game/Blueprints/Saving_and_Loading/SaveGameObject.SaveGameObject_C|GetPlayerData _savegamedata)) false false)
      (Transformation|SetActorLocation _output_get (.location (Variables|/Game/Blueprints/Saving_and_Loading/SaveGameObject.SaveGameObject_C|GetPlayerData _savegamedata)) false false)
      (Variables|/Game/Blueprints/FirstPersonBP/Blueprints/FirstPersonCharacter.FirstPersonCharacter_C|SetHealth _output_get (.health (Variables|/Game/Blueprints/Saving_and_Loading/SaveGameObject.SaveGameObject_C|GetPlayerData _savegamedata)))
      (Variables|/Game/Blueprints/FirstPersonBP/Blueprints/FirstPersonCharacter.FirstPersonCharacter_C|SetProtein _output_get (.food (Variables|/Game/Blueprints/Saving_and_Loading/SaveGameObject.SaveGameObject_C|GetPlayerData _savegamedata)))
      (Variables|/Game/Blueprints/FirstPersonBP/Blueprints/FirstPersonCharacter.FirstPersonCharacter_C|SetWater _output_get (.water (Variables|/Game/Blueprints/Saving_and_Loading/SaveGameObject.SaveGameObject_C|GetPlayerData _savegamedata))))
    (:else)))

(fn ClearSaveData
  (bind _returnvalue (SaveGame|DeleteGameinSlot (Variables|Default|GetSaveSlotName)))
  (if _returnvalue
    (Development|PrintString "Save Cleared")))

(fn AutoSave
  (CallFunction|SavePlayerData)
  (if true
    (Development|PrintString "Autosave")))

(fn RetrieveSaveData
  (params (LOCAL_SaveSlotName :type String))
  (bind _returnvalue (SaveGame|DoesSaveGameExist LOCAL_SaveSlotName))
  (if _returnvalue
    (bind _returnvalue_2 (SaveGame|LoadGamefromSlot LOCAL_SaveSlotName))
    (bind _assave_game_object (Utilities|Casting|CastToSaveGameObject _returnvalue_2))
    (return (Variables|/Game/Blueprints/Saving_and_Loading/SaveGameObject.SaveGameObject_C|GetPlayerData _assave_game_object))))