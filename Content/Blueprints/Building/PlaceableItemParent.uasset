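; Parent actor for placeable building items, moving from preview through placed to built by swapping mesh material and collision.
; Interacting checks the player's inventory against the recipe keys, adds one item to the actor's own inventory, then removes one of each recipe item from the player and refreshes the HUD.
; When that inventory satisfies the recipe, Built restores the default material, blocks pawns and calls the empty DoExtraStuff hook.
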(event Custom|Placed
  (bind _staticmesh (Variables|Default|GetStaticMesh))
  (Rendering|Material|SetMaterial (Variables|Default|GetStaticMesh) 0 "/Game/Blueprints/Building/PreviewMaterialPlaced.PreviewMaterialPlaced")
  (Collision|SetCollisionEnabled _staticmesh "QueryAndPhysics")
  (Collision|SetCollisionResponsetoChannel _staticmesh "ECC_Pawn" "ECR_Ignore"))

(event Custom|Built
  (bind _staticmesh (Variables|Default|GetStaticMesh))
  (Variables|Default|SetIsBuilt true)
  (Rendering|Material|SetMaterial _staticmesh 0 (Variables|Default|GetDefaultMaterial))
  (Collision|SetCollisionEnabled _staticmesh "QueryAndPhysics")
  (Collision|SetCollisionResponsetoChannel _staticmesh "ECC_Pawn" "ECR_Block")
  (CallFunction|DoExtraStuff))

(event Custom|Do%20Extra%20Stuff)

(event EventBeginPlay
  (bind _staticmesh (Variables|Default|GetStaticMesh))
  (bind _asfirst_person_character (Utilities|Casting|CastToFirstPersonCharacter (Game|GetPlayerCharacter 0)))
  (Variables|Default|SetPlayerCharacter _asfirst_person_character)
  (bind _asmy_player_controller (Utilities|Casting|CastToMyPlayerController (Game|GetPlayerController 0)))
  (Variables|Default|SetPlayerController _asmy_player_controller)
  (Variables|Default|SetDefaultMaterial (Rendering|Material|GetMaterial _staticmesh 0))
  (Rendering|Material|SetMaterial _staticmesh 0 "/Game/Blueprints/Building/PreviewMaterial.PreviewMaterial")
  (Collision|SetCollisionEnabled (Variables|Default|GetStaticMesh) "NoCollision")
  (Utilities|FlowControl|Delay 0.5)
  (if (Variables|Default|GetIsBuilt)
    (CallFunction|Built)))

(event EventInteract
  (params (Interacter :type First%20Person%20Character%20Object%20Reference))
  (bind _built (CallFunction|CheckifBuilt self (Variables|Default|GetRecipe)))
  (if (not _built)
    (bind (_success _item) (CallFunction|CheckifItemCanbeAdded (Variables|Default|GetRecipe self)))
    (if _success
      (bind _success_2 (CallFunction|AddtoBuildInventory self _item 1))
      (if _success_2
        (CallFunction|RemovefromInventory self (Variables|Default|GetRecipe) 1)
        (bind _built_2 (CallFunction|CheckifBuilt self (Variables|Default|GetRecipe)))
        (if _built_2
          (CallFunction|Built self))))))

(fn ConstructionScript)

(fn CheckBuildRecipe
  (params (Recipe :type Map%20of%20Item%20Parent%20Class%20References%20to%20Integers))
  (bind _keys (Utilities|Map|Keys Recipe))
  (for _array_element _keys
    (bind (_isininventory _output_quantity _success) (Default|InventoryQueryBuilding (Variables|/Game/Blueprints/FirstPersonBP/Blueprints/FirstPersonCharacter.FirstPersonCharacter_C|GetInventoryComponent (Variables|Default|GetPlayerCharacter)) _array_element (.Value (Utilities|Map|Find Recipe _array_element))))
    (if (not _success)
      (Variables|Default|SetIsComplete false)))
  (return (Variables|Default|GetIsComplete) _output_quantity _array_element))

(fn RemovefromInventory
  (params (BuildItems :type Map%20of%20Item%20Parent%20Class%20References%20to%20Integers) (Quantity :type Integer))
  (bind _playercontroller (Variables|Default|GetPlayerController))
  (bind _hud_widget (Variables|/Game/Blueprints/UI/MyPlayerController.MyPlayerController_C|GetHUD%20Widget _playercontroller))
  (bind _keys (Utilities|Map|Keys BuildItems))
  (for _array_element _keys
    (bind _success (Default|RemovefromInventory (Variables|/Game/Blueprints/FirstPersonBP/Blueprints/FirstPersonCharacter.FirstPersonCharacter_C|GetInventoryComponent (Variables|Default|GetPlayerCharacter)) _array_element Quantity))
    (if _success
      (Default|RefreshInventory (Variables|/Game/Blueprints/UI/HUD.HUD_C|GetInventoryWindow _hud_widget))
      (Default|RefreshInventory (Variables|/Game/Blueprints/UI/HUD.HUD_C|GetCraftingMenu _hud_widget)))))

(fn CheckifBuilt
  (params (BuildItems :type Map%20of%20Item%20Parent%20Class%20References%20to%20Integers))
  (bind _keys (Utilities|Map|Keys BuildItems))
  (for _array_element _keys
    (bind _success (Default|InventoryQuery (Variables|Default|GetInventoryComponent) _array_element (.Value (Utilities|Map|Find BuildItems _array_element))))
    (if (not _success)
      (return false)))
  (return (Variables|Default|GetIsComplete)))

(fn CheckifItemCanbeAdded
  (params (Inventory :type Map%20of%20Item%20Parent%20Class%20References%20to%20Integers))
  (bind _keys (Utilities|Map|Keys Inventory))
  (for _array_element _keys
    (bind _success (Default|InventoryQuery (Variables|/Game/Blueprints/FirstPersonBP/Blueprints/FirstPersonCharacter.FirstPersonCharacter_C|GetInventoryComponent (Variables|Default|GetPlayerCharacter)) _array_element 1))
    (if (not _success)
      (Variables|Default|SetIsComplete false)))
  (return (Variables|Default|GetIsComplete) _array_element))

(fn AddtoBuildInventory
  (params (ItemToBeAdded :type Item%20Parent%20Class%20Reference) (Quantity :type Integer))
  (bind _inventorycomponent (Variables|Default|GetInventoryComponent))
  (bind _inventory2 (Variables|/Game/Blueprints/UI/Inventory/InventoryComponent.InventoryComponent_C|GetInventory2 _inventorycomponent))
  (Utilities|Map|Add _inventory2 ItemToBeAdded (Math|Integer|Clamp(Integer) (+ Quantity (.Value (Utilities|Map|Find _inventory2 ItemToBeAdded))) 0 20))
  (return true))