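; Base Blueprint for an Alaskan cedar tree actor that tracks health and can be replaced by another tree actor.
; TakeDamage subtracts Damage from Health without checking the result.
; The depletion check runs only in BeginPlay: at zero or less Health, the actor destroys itself and spawns its TreeType class at the same transform.
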(event EventBeginPlay
  (if (<= (Variables|Default|GetHealth) 0.0)
    (Actor|DestroyActor)
    (Game|SpawnActorfromClass (Variables|Default|GetTreeType) (Transformation|GetActorTransform) "Undefined" 0 0)))

(event Collision|EventActorBeginOverlap
  (params (OtherActor :type Actor%20Object%20Reference)))

(event EventTick
  (params (DeltaSeconds :type Float%20%28single-precision%29)))

(fn ConstructionScript)

(fn TakeDamage
  (Variables|Default|SetHealth (- (Variables|Default|GetHealth) (Variables|Default|GetDamage))))