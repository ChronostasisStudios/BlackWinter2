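; Base class for world items that can be picked up into an inventory, applying mesh and scale from class defaults on BeginPlay.
; Interact adds the item's class and gather amount to the interacter's InventoryComponent, then on success refreshes inventory and crafting widgets and destroys the actor.
; UseItem is a stub returning false.
; FoodStats adds health, water, protein, carb and fat values to the player character, clamped between zero and one.
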(event EventBeginPlay
  (bind _self self)
  (bind _staticmesh (Variables|Default|GetStaticMesh))
  (bind _staticmesh_2 (Variables|Default|GetStaticMesh))
  (bind _returnvalue (Utilities|GetClass _self))
  (bind (_category _iscraftable _name _description _thumbnail _crafting_recipe _craftingoutput _gatheramount _isconsumable _mesh _scale) (Utilities|GetClassDefaults _returnvalue))
  (Variables|Default|SetMesh (Variables|/Script/Engine.StaticMeshComponent|GetStaticMesh _staticmesh_2))
  (Components|StaticMesh|SetStaticMesh _staticmesh _mesh)
  (Rendering|Material|SetMaterial _staticmesh 0 (Rendering|Material|GetMaterial _staticmesh_2 0))
  (Transformation|SetWorldScale3D _staticmesh _scale))

(event EventInteract
  (params (Interacter :type First%20Person%20Character%20Object%20Reference))
  (bind _success (Default|AddtoInventory (Variables|/Game/Blueprints/FirstPersonBP/Blueprints/FirstPersonCharacter.FirstPersonCharacter_C|GetInventoryComponent Interacter) (Utilities|GetClass self) (Variables|Default|GetGatherAmount)))
  (if _success
    (bind _asmy_player_controller (Utilities|Casting|CastToMyPlayerController (Game|GetPlayerController 0)))
    (Default|RefreshInventory (Variables|/Game/Blueprints/UI/HUD.HUD_C|GetInventoryWindow (Variables|/Game/Blueprints/UI/MyPlayerController.MyPlayerController_C|GetHUD%20Widget _asmy_player_controller)))
    (Default|RefreshInventory (Variables|/Game/Blueprints/UI/HUD.HUD_C|GetCraftingMenu (Variables|/Game/Blueprints/UI/MyPlayerController.MyPlayerController_C|GetHUD%20Widget _asmy_player_controller)))
    (Actor|DestroyActor)))

(fn ConstructionScript)

(fn UseItem
  (return false))

(fn FoodStats
  (params (HealthStat :type Float%20%28single-precision%29) (WaterStat :type Float%20%28single-precision%29) (ProteinStat :type Float%20%28single-precision%29) (CarbStat :type Float%20%28single-precision%29) (FatStat :type Float%20%28single-precision%29))
  (bind _asfirst_person_character (Utilities|Casting|CastToFirstPersonCharacter (Game|GetPlayerCharacter 0)))
  (Variables|/Game/Blueprints/FirstPersonBP/Blueprints/FirstPersonCharacter.FirstPersonCharacter_C|SetHealth _asfirst_person_character (Math|Float|Clamp(Float) (+ (Variables|/Game/Blueprints/FirstPersonBP/Blueprints/FirstPersonCharacter.FirstPersonCharacter_C|GetHealth _asfirst_person_character) HealthStat)))
  (Variables|/Game/Blueprints/FirstPersonBP/Blueprints/FirstPersonCharacter.FirstPersonCharacter_C|SetWater _asfirst_person_character (Math|Float|Clamp(Float) (+ (Variables|/Game/Blueprints/FirstPersonBP/Blueprints/FirstPersonCharacter.FirstPersonCharacter_C|GetWater _asfirst_person_character) WaterStat)))
  (Variables|/Game/Blueprints/FirstPersonBP/Blueprints/FirstPersonCharacter.FirstPersonCharacter_C|SetProtein _asfirst_person_character (Math|Float|Clamp(Float) (+ (Variables|/Game/Blueprints/FirstPersonBP/Blueprints/FirstPersonCharacter.FirstPersonCharacter_C|GetProtein _asfirst_person_character) ProteinStat)))
  (Variables|/Game/Blueprints/FirstPersonBP/Blueprints/FirstPersonCharacter.FirstPersonCharacter_C|SetCarbs _asfirst_person_character (Math|Float|Clamp(Float) (+ (Variables|/Game/Blueprints/FirstPersonBP/Blueprints/FirstPersonCharacter.FirstPersonCharacter_C|GetCarbs _asfirst_person_character) CarbStat)))
  (Variables|/Game/Blueprints/FirstPersonBP/Blueprints/FirstPersonCharacter.FirstPersonCharacter_C|SetFats _asfirst_person_character (Math|Float|Clamp(Float) (+ (Variables|/Game/Blueprints/FirstPersonBP/Blueprints/FirstPersonCharacter.FirstPersonCharacter_C|GetFats _asfirst_person_character) FatStat)))
  (return))